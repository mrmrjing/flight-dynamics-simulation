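; Flight sim Blueprint that lets the player fly a Plane static mesh with keyboard controls.
; W and S step thrust per press, floored at zero and printed, while held A/D and Q/E set flags for pitch and roll.
; Tick applies fixed rotation increments without delta-time scaling, then feeds thrust and hard-coded aerodynamic coefficients into FlightSimulation.
; Each tick ends by forcing world yaw to a constant, locking the heading.
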(event `Key|D`
  (params (Key :type "Key Structure"))
  (:`Pressed`
    (set `self.isPressedD` true))
  (:`Released`
    (set `self.isPressedD` false)))

(event `Key|W`
  (params (Key :type "Key Structure"))
  (:`Pressed`
    (set `self.Thrust` (+ (`self.Thrust`) (`self.ThrustIncremenet`)))
    (`KismetSystemLibrary.PrintString` (`KismetStringLibrary.Conv_DoubleToString` (`self.Thrust`)) :!label _label)))

(event `Key|A`
  (params (Key :type "Key Structure"))
  (:`Pressed`
    (set `self.isPressedA` true))
  (:`Released`
    (set `self.isPressedA` false)))

(event `Key|Q`
  (params (Key :type "Key Structure"))
  (:`Pressed`
    (set `self.isPressedQ` true))
  (:`Released`
    (set `self.isPressedQ` false)))

(event `Key|S`
  (params (Key :type "Key Structure"))
  (bind _returnvalue (- (`self.Thrust`) (`self.ThrustIncremenet`)))
  (:`Pressed`
    (if (< _returnvalue 0.0)
      (set `self.Thrust` 0.0)
      (goto _label)
      (else
        (set `self.Thrust` _returnvalue)
        (goto _label)))))

(event `Key|E`
  (params (Key :type "Key Structure"))
  (:`Pressed`
    (set `self.isPressedE` true))
  (:`Released`
    (set `self.isPressedE` false)))

(event `self.ReceiveTick`
  (params (DeltaSeconds :type "Float (single-precision)"))
  (bind _pitchincremenet (`self.PitchIncremenet`))
  (bind _rollincremenet (`self.RollIncremenet`))
  (bind (_returnvalue_roll _returnvalue_pitch _returnvalue_yaw) (`KismetMathLibrary.BreakRotator` (`SceneComponent.K2_GetComponentRotation` (`self.Plane`))))
  (bind (_returnvalue_roll_2 _returnvalue_pitch_2) (`KismetMathLibrary.BreakRotator` (`SceneComponent.K2_GetComponentRotation` (`self.Plane`))))
  (bind (_returnvalue_roll_3 _returnvalue_pitch_3 _returnvalue_yaw_2) (`KismetMathLibrary.BreakRotator` (`SceneComponent.K2_GetComponentRotation` (`self.Plane`))))
  (if (`self.isPressedA`)
    (`SceneComponent.K2_SetWorldRotation` (`self.Plane`) (`KismetMathLibrary.MakeRotator` _returnvalue_roll_3 (- _returnvalue_pitch_3 _pitchincremenet) _returnvalue_yaw_2) false false))
  (if (`self.isPressedD`)
    (`SceneComponent.K2_SetWorldRotation` (`self.Plane`) (`KismetMathLibrary.MakeRotator` _returnvalue_roll_3 (+ _returnvalue_pitch_3 _pitchincremenet) _returnvalue_yaw_2) false false))
  (if (`self.isPressedQ`)
    (`SceneComponent.K2_SetWorldRotation` (`self.Plane`) (`KismetMathLibrary.MakeRotator` (+ _returnvalue_roll _rollincremenet) _returnvalue_pitch _returnvalue_yaw) false false))
  (if (`self.isPressedE`)
    (`SceneComponent.K2_SetWorldRotation` (`self.Plane`) (`KismetMathLibrary.MakeRotator` (- _returnvalue_roll _rollincremenet) _returnvalue_pitch _returnvalue_yaw) false false))
  (`FlightSimPluginBPLibrary.FlightSimulation` self (`self.Plane`) true 2.0 0.8 1.0 2.0 (`self.Thrust`))
  (`SceneComponent.K2_SetWorldRotation` (`self.Plane`) (`KismetMathLibrary.MakeRotator` _returnvalue_roll_2 _returnvalue_pitch_2 270.0) false false))

(fn `UserConstructionScript`)